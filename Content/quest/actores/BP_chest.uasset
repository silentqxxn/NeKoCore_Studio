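; BP_chest is a quest chest actor that identifies itself to interaction as the non-NPC objective "ChestMision1" through InteractWith.
; Its Interactuar event checks for a valid character and a not-yet-open chest, but nothing follows those checks.
; A separate AnadirItemAlJugador event, not called in this graph, has a weighted random chance to set the character's ArmaActual to None, so no item is actually granted.
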(event Custom|AnadirItemAlJugador
  (params (character :type BP%20Character%20Object%20Reference))
  (if (Math|Random|RandomBoolwithWeight 0.3)
    (Variables|/Game/Characters/BP_Character.BP_Character_C|SetArmaActual character 0)))

(event EventBeginPlay)

(event Collision|EventActorBeginOverlap
  (params (OtherActor :type Actor%20Object%20Reference)))

(event EventTick
  (params (DeltaSeconds :type Float%20%28single-precision%29)))

(event EventInteractuar
  (params (character :type BP%20Character%20Object%20Reference))
  (Utilities|IsValid character
    (:Is%20Valid
      (if (not (Variables|Default|Getesta%20abierto?))
        _))))

(fn ConstructionScript)

(fn Interactwith
  (return (Utilities|String|StringToName (Utilities|String|MakeLiteralString "ChestMision1")) false))