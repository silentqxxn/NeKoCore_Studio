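; Base quest actor that tracks one quest's objectives through ComponenteMisiones on the player state, using stage data from DT_QuestData.
; BeginPlay calls ProgressObjective with the first stage's type and required amount, while GetQuestDeatails caches the current stage.
; OnObjetiveIDHeard adds progress and checks stage completion.
; If the whole quest is then complete, ObjetivoCompletado shows a notification, sets IsCompleted and awards the stage's bonus XP.
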(event EventBeginPlay
  (bind _asplayer_state_countless_blood (Utilities|Casting|CastToPlayerStateCountlessBlood (Variables|/Script/Engine.Pawn|GetPlayerState (CallFunction|GetMyPlayerCharacter))))
  (bind _returnvalue (Utilities|GetDataTableRow "/Game/Datatable/DT_QuestData.DT_QuestData" (Variables|Default|GetQuestID))
    (:then
      (Class|ComponenteMisiones|ProgressObjective (Variables|/Script/proyectoejercicio.PlayerStateCountlessBlood|GetComponenteMisiones _asplayer_state_countless_blood) (Variables|Default|GetQuestID) (.TipoObjetivo (Utilities|Struct|BreakQuestStage (Utilities|Array|Get(acopy) (.Stages (Utilities|Struct|BreakQuestData _returnvalue))))) (.CantidadRequerida (Utilities|Struct|BreakQuestStage (Utilities|Array|Get(acopy) (.Stages (Utilities|Struct|BreakQuestData _returnvalue)))))))))

(event Collision|EventActorBeginOverlap
  (params (OtherActor :type Actor%20Object%20Reference)))

(event EventTick
  (params (DeltaSeconds :type Float%20%28single-precision%29)))

(fn ConstructionScript)

(fn OnObjetiveIDHeard
  (params (ObjetiveID :type Name) (Value :type Integer))
  (bind _currentstagedetalles (Variables|Default|GetCurrentStageDetalles))
  (bind (_objectiveid _objectivename _description _tipoobjetivo) (Utilities|Struct|BreakQuestStage _currentstagedetalles))
  (bind _asplayer_state_countless_blood (Utilities|Casting|CastToPlayerStateCountlessBlood (Variables|/Script/Engine.Pawn|GetPlayerState (CallFunction|GetMyPlayerCharacter))))
  (Class|ComponenteMisiones|ProgressObjective (Variables|/Script/proyectoejercicio.PlayerStateCountlessBlood|GetComponenteMisiones _asplayer_state_countless_blood) ObjetiveID _tipoobjetivo Value)
  (if (Class|ComponenteMisiones|IsObjectiveStageComplete (Variables|/Script/proyectoejercicio.PlayerStateCountlessBlood|GetComponenteMisiones _asplayer_state_countless_blood) _objectiveid)
    (CallFunction|ObjetivoCompletado ObjetiveID)
    (return)))

(fn GetQuestDeatails
  (bind _returnvalue (Utilities|GetDataTableRow "/Game/Datatable/DT_QuestData.DT_QuestData" (Variables|Default|GetQuestID))
    (:then
      (Variables|Default|SetCurrentStageDetalles (Utilities|Array|Get(acopy) (.Stages (Utilities|Struct|BreakQuestData _returnvalue)) (Variables|Default|GetCurrentStage)))
      (return))))

(fn GetObjetiveDatabyID
  (params (ObjetiveID :type Name))
  (bind _currentstagedetalles (Variables|Default|GetCurrentStageDetalles))
  (if (== (.ObjectiveID (Utilities|Struct|BreakQuestStage _currentstagedetalles)) ObjetiveID)
    (return _currentstagedetalles)))

(fn ObjetivoCompletado
  (params (ObjetiveID :type Name))
  (bind _queststagearray (CallFunction|GetObjetiveDatabyID ObjetiveID))
  (bind (_objectiveid _objectivename _description _tipoobjetivo _cantidadrequerida _bisoptional _bonusxp) (Utilities|Struct|BreakQuestStage _queststagearray))
  (bind _asplayer_state_countless_blood (Utilities|Casting|CastToPlayerStateCountlessBlood (Variables|/Script/Engine.Pawn|GetPlayerState (CallFunction|GetMyPlayerCharacter))))
  (if (Class|ComponenteMisiones|IsQuestCompleted (Variables|/Script/proyectoejercicio.PlayerStateCountlessBlood|GetComponenteMisiones _asplayer_state_countless_blood) (Variables|Default|GetQuestID))
    (bind _returnvalue (UserInterface|CreateWidget "/Game/ui/questUI/WBP_NotificaciónMision.WBP_NotificaciónMision_C" 0 _description))
    (UserInterface|Viewport|AddtoViewport _returnvalue 0)
    (bind _return (CallFunction|MisionCompletada))
    (Variables|Default|SetIsCompleted _return)
    (Class|BPIExperiencia|ObtenerExperiencia(Message) (Game|GetPlayerCharacter 0) _bonusxp)))

(fn MisionCompletada
  (bind _asplayer_state_countless_blood (Utilities|Casting|CastToPlayerStateCountlessBlood (Variables|/Script/Engine.Pawn|GetPlayerState (CallFunction|GetMyPlayerCharacter)))
    (:then
      (return (Class|ComponenteMisiones|IsQuestCompleted (Variables|/Script/proyectoejercicio.PlayerStateCountlessBlood|GetComponenteMisiones _asplayer_state_countless_blood) (Variables|Default|GetQuestID))))
    (:CastFailed
      (return false))))