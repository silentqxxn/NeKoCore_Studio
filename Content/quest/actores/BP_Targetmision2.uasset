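; BP_Targetmision2 is a damageable enemy target that advances a quest objective when killed.
; GolpeVampiro subtracts damage from BPComponenteVida and refreshes the enemy health bar widget, using a fixed maximum.
; The death check subtracts the damage a second time, then reports ObjetiveID to BP_Character, grants the player experience and destroys the actor.
; AnyDamage is empty, and older Healt-based damage logic is left disconnected.
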(event EventBeginPlay
  (|CallParentFunction))

(event Collision|EventActorBeginOverlap
  (params (OtherActor :type Actor%20Object%20Reference))
  (|CallParentFunction OtherActor))

(event EventSaludInicialEnemigo
  (params (Vida :type Float%20%28double-precision%29) (Vida%20max :type Float%20%28double-precision%29))
  (bind _aswbp_barra_vida_enemigo (Utilities|Casting|CastToWBP_BarraVidaEnemigo (UserInterface|GetWidget (Variables|Default|GetWidget))))
  (Variables|Default|SetAs%20WBP%20Barra%20Vida%20Enemigo _aswbp_barra_vida_enemigo)
  (CallFunction|ActualizarWidgetenemigo Vida Vida%20max))

(event EventTick
  (params (DeltaSeconds :type Float%20%28single-precision%29))
  (|CallParentFunction DeltaSeconds))

(event Game|Damage|EventAnyDamage
  (params (Damage :type Float%20%28single-precision%29) (DamageType :type Damage%20Type%20Object%20Reference) (InstigatedBy :type Controller%20Object%20Reference) (DamageCauser :type Actor%20Object%20Reference)))

(event EventEnemigoRecibioDano
  (params (Vida :type Float%20%28double-precision%29) (Vida%20max :type Float%20%28double-precision%29))
  (CallFunction|ActualizarWidgetenemigo Vida Vida%20max))

(event EventGolpeVampiro
  (params (daño :type Float%20%28double-precision%29))
  (bind _returnvalue (Game|GetPlayerCharacter 0))
  (bind _bp_componentevida (Variables|Default|GetBP_ComponenteVida))
  (bind _output_get (Variables|/Game/componente/BP_ComponenteVida.BP_ComponenteVida_C|SetVida _bp_componentevida (- (Variables|/Game/componente/BP_ComponenteVida.BP_ComponenteVida_C|GetVida _bp_componentevida) daño)))
  (CallFunction|EnemigoRecibioDano _output_get 1e+02)
  (if (<= (- (Variables|/Game/componente/BP_ComponenteVida.BP_ComponenteVida_C|GetVida _bp_componentevida) daño) 0.0)
    (bind _asbp_character (Utilities|Casting|CastToBP_Character _returnvalue))
    (Default|CallOnObjetiveID _asbp_character (Variables|Default|GetObjetiveID) 1)
    (Class|BPIExperiencia|ObtenerExperiencia(Message) _returnvalue 15.0)
    (Actor|DestroyActor)))

(fn ConstructionScript)

(fn ActualizarWidgetenemigo
  (params (vida :type Float%20%28double-precision%29) (vidamax :type Float%20%28double-precision%29))
  (Progress|SetPercent (Variables|/Game/ui/BarraVidaEnemigo/WBP_BarraVidaEnemigo.WBP_BarraVidaEnemigo_C|GetProgressBar_vidaenemigo (Variables|Default|GetAs%20WBP%20Barra%20Vida%20Enemigo)) (/ vida vidamax)))