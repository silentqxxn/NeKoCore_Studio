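; Player controller that creates the local player's main HUD and mission window UI.
; On BeginPlay it adds both widgets to the viewport, with the mission window starting hidden.
; The IA_TablaMisiones input toggles that window, refreshing its list and switching input mode and mouse cursor between game-only and game-and-UI.
; Disconnected nodes for an ammo widget remain in the graph and never run.
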(event Input|EnhancedActionEvents|EnhancedInputActionIA_TablaMisiones
  (params (ActionValue :type Boolean) (ElapsedSeconds :type Float%20%28double-precision%29) (TriggeredSeconds :type Float%20%28double-precision%29) (InputAction :type Input%20Action%20Object%20Reference :default "/Game/imputs/IA_TablaMisiones.IA_TablaMisiones"))
  (bind _ref_menumisiones (Variables|Default|GetRef_MenuMisiones))
  (bind _ref_menumisiones_2 (Variables|Default|GetRef_MenuMisiones))
  (:Started
    (if (== (Widget|GetVisibility (Variables|Default|GetRef_MenuMisiones)) 0)
      (Widget|SetVisibility _ref_menumisiones_2 "Hidden")
      (Default|RefrescarLista _ref_menumisiones_2)
      (Input|SetInputModeGameOnly self false)
      (Variables|Default|SetbShowMouseCursor false)
      (else
        (Utilities|IsValid (Variables|Default|GetRef_MenuMisiones)
          (:Is%20Valid
            (Widget|SetVisibility _ref_menumisiones "Visible")
            (Default|RefrescarLista _ref_menumisiones)
            (Input|SetInputModeGameandUI self 0 "DoNotLock" true false)
            (Variables|Default|SetbShowMouseCursor true)))))))

(event EventBeginPlay
  (if (Pawn|IsLocalPlayerController)
    (bind _returnvalue (UserInterface|CreateWidget "/Game/ui/WBP_ui.WBP_ui_C"))
    (bind _output_get (Variables|Default|SetRef_HUD_Principal _returnvalue))
    (UserInterface|Viewport|AddtoViewport _output_get 0)
    (bind _returnvalue_2 (UserInterface|CreateWidget "/Game/ui/questUI/WBP_VentanaMisiones.WBP_VentanaMisiones_C"))
    (bind _output_get_2 (Variables|Default|SetRef_MenuMisiones _returnvalue_2))
    (UserInterface|Viewport|AddtoViewport _output_get_2 0)
    (Widget|SetVisibility _output_get_2 "Hidden")))

(event EventTick
  (params (DeltaSeconds :type Float%20%28single-precision%29)))

(fn ConstructionScript)