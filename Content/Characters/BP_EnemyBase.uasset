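; Base enemy character that manages a health bar, vampire-hit damage and death rewards.
; BPComponenteVida events update the widget bar, while GolpeVampiro subtracts health directly and refreshes it manually.
; At zero health it advances the attacker's kill quest, then a DoOnce plays the death animation, grants experience and destroys the actor.
; DisparoMonjaBase spawns a targeted projectile, but its montage-driven caller is disconnected and AtaqueDistancia is empty.
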(event Custom|SaludInicialEnemigo
  (params (Vida :type Float%20%28double-precision%29) (Vida%20max :type Float%20%28double-precision%29))
  (Default|ActualizarVidaEnemigo (Variables|Default|Getbarravidaenemigo) Vida Vida%20max))

(event Custom|EnemigoRecibioDano
  (params (Vida :type Float%20%28double-precision%29) (Vida%20max :type Float%20%28double-precision%29))
  (Default|ActualizarVidaEnemigo (Variables|Default|Getbarravidaenemigo) Vida Vida%20max))

(event Custom|EnemigoCurandose
  (params (Vida :type Float%20%28double-precision%29) (VidaMax :type Float%20%28double-precision%29))
  (Default|ActualizarVidaEnemigo (Variables|Default|Getbarravidaenemigo) Vida VidaMax))

(event EventBeginPlay
  (bind _bp_componentevida (Variables|Default|GetBP_ComponenteVida))
  (bind _aswbp_barra_vida_enemigo (Utilities|Casting|CastToWBP_BarraVidaEnemigo (UserInterface|GetUserWidgetObject (Variables|Default|GetWidget))))
  (bind _output_get (Variables|Default|Setbarravidaenemigo _aswbp_barra_vida_enemigo))
  (CallFunction|ActuiEnemigo _output_get)
  (EventDispatchers|BindEventtoSaludIni _bp_componentevida (delegate Custom|SaludInicialEnemigo))
  (EventDispatchers|BindEventtoRecibiDano _bp_componentevida (delegate Custom|EnemigoRecibioDano))
  (EventDispatchers|BindEventtoCuracion _bp_componentevida (delegate Custom|EnemigoCurandose)))

(event Collision|EventActorBeginOverlap
  (params (OtherActor :type Actor%20Object%20Reference)))

(event EventTick
  (params (DeltaSeconds :type Float%20%28single-precision%29)))

(event EventGolpeVampiro
  (params (daño :type Float%20%28double-precision%29) (Atacante :type BP%20Character%20Object%20Reference))
  (bind _bp_componentevida (Variables|Default|GetBP_ComponenteVida))
  (bind _output_get (Variables|/Game/componente/BP_ComponenteVida.BP_ComponenteVida_C|SetVida _bp_componentevida (- (Variables|/Game/componente/BP_ComponenteVida.BP_ComponenteVida_C|GetVida _bp_componentevida) daño)))
  (CallFunction|EnemigoRecibioDano _output_get (Variables|/Game/componente/BP_ComponenteVida.BP_ComponenteVida_C|GetVida%20max _bp_componentevida))
  (if (<= _output_get 0.0)
    (bind _asbp_player_state_countless_blood (Utilities|Casting|CastToBP_PlayerStateCountlessBlood (Variables|/Script/Engine.Pawn|GetPlayerState Atacante)))
    (Class|ComponenteMisiones|ProgressObjective (Variables|/Script/proyectoejercicio.PlayerStateCountlessBlood|GetComponenteMisiones _asbp_player_state_countless_blood) "M10001" "Matar" 1)
    (Utilities|FlowControl|DoOnce false
      (:Completed
        (Components|Animation|PlayAnimation (Variables|Character|GetMesh) (Variables|Default|GetAnimacionmuerte) false)
        (Utilities|FlowControl|Delay 1.0)
        (Class|BPIExperiencia|ObtenerExperiencia(Message) Atacante (Variables|Default|GetExperiencia))
        (Actor|DestroyActor)))))

(event EventAtaqueDistancia)

(fn ConstructionScript)

(fn ActuiEnemigo
  (params (barravidaenemigo :type WBP%20Barra%20Vida%20Enemigo%20Object%20Reference))
  (bind _bp_componentevida (Variables|Default|GetBP_ComponenteVida))
  (bind _output_get (Variables|Default|Setbarravidaenemigo barravidaenemigo))
  (Utilities|IsValid barravidaenemigo
    (:Is%20Valid
      (Progress|SetPercent (Variables|/Game/ui/BarraVidaEnemigo/WBP_BarraVidaEnemigo.WBP_BarraVidaEnemigo_C|GetProgressBar_vidaenemigo _output_get) (/ (Variables|/Game/componente/BP_ComponenteVida.BP_ComponenteVida_C|GetVida _bp_componentevida) (Variables|/Game/componente/BP_ComponenteVida.BP_ComponenteVida_C|GetVida%20max _bp_componentevida))))))

(fn DisparoMonjaBase
  (params (Objetivo :type BP%20Character%20Object%20Reference))
  (Variables|Default|SetObjetivo Objetivo)
  (Game|SpawnActorfromClass "/Game/Characters/EnemigoDistancia/BP_Proyectil.BP_Proyectil_C" (Transformation|GetActorTransform) "Undefined" "MultiplyWithRoot" 0 (Variables|Default|GetVelocidad%20Proyectil) (Variables|Default|GetDaño%20Proyectil) (Variables|Default|GetObjetivo) 0))