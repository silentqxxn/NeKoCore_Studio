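; Melee vampire enemy, a child Blueprint that targets the player on BeginPlay and sets its own death animation.
; Health events feed the percentage of an overhead-style health bar widget.
; AtaqueMonja plays a punch montage, then immediately sphere-traces at the right-hand socket and applies damage through an interface, without waiting for the animation notify.
; Older damage, objective-reporting and destroy logic remains unconnected.
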(event OnComponentBeginOverlap(HitBox)
  (params (OverlappedComponent :type Primitive%20Component%20Object%20Reference) (OtherActor :type Actor%20Object%20Reference) (OtherComp :type Primitive%20Component%20Object%20Reference) (OtherBodyIndex :type Integer) (bFromSweep :type Boolean) (SweepResult :type Hit%20Result%20Structure%20%28by%20ref%29)))

(event Custom|Multicas_animAtaqueMele
  (Animation|Montage|PlayMontage (Variables|Character|GetMesh) "/Game/Characters/enemigoMele/Mutant_Punch_Montage.Mutant_Punch_Montage"
    (:then
      _)
    (:OnNotifyBegin
      _))
  (Variables|Default|SetEstaAtacando? true)
  (Utilities|FlowControl|Delay 1.0))

(event EventBeginPlay
  (|CallParentFunction)
  (CallFunction|SetTarget (CallFunction|GetMyPlayerCharacter))
  (Variables|Default|SetAnimacionmuerte "/Game/Characters/enemigoMele/Standing_React_Death_Backward.Standing_React_Death_Backward"))

(event Collision|EventActorBeginOverlap
  (params (OtherActor :type Actor%20Object%20Reference))
  (|CallParentFunction OtherActor) ; This node is disabled and will not be called.\nDrag off pins to build functionality.
)

(event EventTick
  (params (DeltaSeconds :type Float%20%28single-precision%29))
  (|CallParentFunction DeltaSeconds) ; This node is disabled and will not be called.\nDrag off pins to build functionality.
)

(event EventSaludInicialEnemigo
  (params (Vida :type Float%20%28double-precision%29) (Vida%20max :type Float%20%28double-precision%29))
  (bind _aswbp_barra_vida_enemigo (Utilities|Casting|CastToWBP_BarraVidaEnemigo (UserInterface|GetWidget (Variables|Default|GetWidget))))
  (Variables|Default|SetAs%20WBP%20Barra%20Vida%20Enemigo _aswbp_barra_vida_enemigo)
  (CallFunction|ActualizarWidgetenemigo Vida Vida%20max))

(event EventAtaqueMonja
  (CallFunction|MulticasAnimAtaqueMele)
  (CallFunction|HitDetect)
  (Variables|Default|SetEstaAtacando? false))

(event EventEnemigoRecibioDano
  (params (Vida :type Float%20%28double-precision%29) (Vida%20max :type Float%20%28double-precision%29))
  (CallFunction|ActualizarWidgetenemigo Vida Vida%20max))

(fn ConstructionScript
  (|CallParentFunction))

(fn ActualizarWidgetenemigo
  (params (vida :type Float%20%28double-precision%29) (vidamax :type Float%20%28double-precision%29))
  (Progress|SetPercent (Variables|/Game/ui/BarraVidaEnemigo/WBP_BarraVidaEnemigo.WBP_BarraVidaEnemigo_C|GetProgressBar_vidaenemigo (Variables|Default|GetAs%20WBP%20Barra%20Vida%20Enemigo)) (/ vida vidamax)))

(fn SetTarget
  (params (Target :type BP%20Character%20Object%20Reference))
  (Variables|Default|SetTarget Target))

(fn HitDetect
  (bind _mesh (Variables|Character|GetMesh))
  (bind _returnvalue (Transformation|GetSocketLocation _mesh "Hand_R"))
  (bind _outhit (Collision|SphereTraceForObjects _returnvalue _returnvalue 3e+01 (Utilities|Array|MakeArray "ObjectTypeQuery7") false 0 "ForDuration"))
  (if (Utilities|DoesObjectImplementInterface (.HitActor (Collision|BreakHitResult _outhit)) "/Script/proyectoejercicio.interfazparahacerdanio")
    (Class|Interfazparahacerdanio|RealizarDanio(Message) (.HitActor (Collision|BreakHitResult _outhit)) (Variables|Default|GetDanio))))