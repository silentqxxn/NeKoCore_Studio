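; BP_EnemigoMele is a melee enemy character with an overhead or attached widget health bar.
; Health events cache the WBP_BarraVidaEnemigo widget and set its progress bar from current over maximum health.
; HitBox overlaps send the enemy's damage to the other actor through a DanoesferaMessage call.
; An unconnected chain that would update health, report objective progress to BP_Character and destroy the enemy never runs.
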(event OnComponentBeginOverlap(HitBox)
  (params (OverlappedComponent :type Primitive%20Component%20Object%20Reference) (OtherActor :type Actor%20Object%20Reference) (OtherComp :type Primitive%20Component%20Object%20Reference) (OtherBodyIndex :type Integer) (bFromSweep :type Boolean) (SweepResult :type Hit%20Result%20Structure%20%28by%20ref%29))
  (Class|BPIDano|Danoesfera(Message) OtherActor (Variables|Default|GetDaño)))

(event EventBeginPlay
  (|CallParentFunction) ; This node is disabled and will not be called.\nDrag off pins to build functionality.
)

(event Collision|EventActorBeginOverlap
  (params (OtherActor :type Actor%20Object%20Reference))
  (|CallParentFunction OtherActor) ; This node is disabled and will not be called.\nDrag off pins to build functionality.
)

(event EventTick
  (params (DeltaSeconds :type Float%20%28single-precision%29))
  (|CallParentFunction DeltaSeconds) ; This node is disabled and will not be called.\nDrag off pins to build functionality.
)

(event EventSaludInicialEnemigo
  (params (Vida :type Float%20%28double-precision%29) (Vida%20max :type Float%20%28double-precision%29))
  (bind _aswbp_barra_vida_enemigo (Utilities|Casting|CastToWBP_BarraVidaEnemigo (UserInterface|GetWidget (Variables|Default|GetWidget))))
  (Variables|Default|SetAs%20WBP%20Barra%20Vida%20Enemigo _aswbp_barra_vida_enemigo)
  (CallFunction|ActualizarWidgetenemigo Vida Vida%20max))

(event EventEnemigoRecibioDano
  (params (Vida :type Float%20%28double-precision%29) (Vida%20max :type Float%20%28double-precision%29))
  (CallFunction|ActualizarWidgetenemigo Vida Vida%20max))

(fn ConstructionScript
  (|CallParentFunction))

(fn ActualizarWidgetenemigo
  (params (vida :type Float%20%28double-precision%29) (vidamax :type Float%20%28double-precision%29))
  (Progress|SetPercent (Variables|/Game/ui/BarraVidaEnemigo/WBP_BarraVidaEnemigo.WBP_BarraVidaEnemigo_C|GetProgressBar_vidaenemigo (Variables|Default|GetAs%20WBP%20Barra%20Vida%20Enemigo)) (/ vida vidamax)))