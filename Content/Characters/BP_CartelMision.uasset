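; BP_CartelMision is a mission sign that starts a co-op mission when a BP_Character enters its ZonaMision trigger.
; On the server, it records the character in JugadoresEnZona and checks GS_CoopMision, calling MisionCompletadaMulticas if the mission is already complete.
; Otherwise, the first entry sets MisionActivada and calls ClienteMostrarContador on that character only.
; End overlap is empty, so players are never removed from the list.
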(event OnComponentBeginOverlap(ZonaMision)
  (params (OverlappedComponent :type Primitive%20Component%20Object%20Reference) (OtherActor :type Actor%20Object%20Reference) (OtherComp :type Primitive%20Component%20Object%20Reference) (OtherBodyIndex :type Integer) (bFromSweep :type Boolean) (SweepResult :type Hit%20Result%20Structure%20%28by%20ref%29))
  (Development|PrintString "Hello")
  (Networking|SwitchHasAuthority
    (:Authority
      (bind _asbp_character (Utilities|Casting|CastToBP_Character OtherActor))
      (Utilities|Array|AddUnique (Variables|Default|GetJugadoresEnZona) _asbp_character)
      (bind _asgs_coop_mision (Utilities|Casting|CastToGS_CoopMision (Game|GetGameState)))
      (if (Variables|/Game/Characters/GS_CoopMision.GS_CoopMision_C|GetMisionCompletada _asgs_coop_mision)
        (Default|MisionCompletadaMulticas _asgs_coop_mision)
        (elif (not (Variables|/Game/Characters/GS_CoopMision.GS_CoopMision_C|GetMision%20Activada _asgs_coop_mision))
          (Variables|/Game/Characters/GS_CoopMision.GS_CoopMision_C|SetMision%20Activada _asgs_coop_mision true)
          (Default|ClienteMostrarContador _asbp_character)
          (if (Variables|/Game/Characters/GS_CoopMision.GS_CoopMision_C|GetMision%20Activada _asgs_coop_mision)
            (Development|PrintText "MISION ACTIVA_1")))))))

(event OnComponentEndOverlap(ZonaMision)
  (params (OverlappedComponent :type Primitive%20Component%20Object%20Reference) (OtherActor :type Actor%20Object%20Reference) (OtherComp :type Primitive%20Component%20Object%20Reference) (OtherBodyIndex :type Integer)))

(event EventBeginPlay)

(event Collision|EventActorBeginOverlap
  (params (OtherActor :type Actor%20Object%20Reference)))

(event EventTick
  (params (DeltaSeconds :type Float%20%28single-precision%29)))

(fn ConstructionScript)