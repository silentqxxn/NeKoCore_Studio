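; BP_Fogata is a campfire actor where the player saves progress and opens the crafting menu.
; Its Sphere overlap enables input and sets TeclaC only for a locally controlled BP_Character, then reverses both on exit.
; The C key drives a FlipFlop that either calls ServerGuardarProgreso and shows WBP_Crafteo with mouse cursor, or removes the widget and restores game-only input.
; Leaving the sphere does not close an open menu.
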(event OnComponentBeginOverlap(Sphere)
  (params (OverlappedComponent :type Primitive%20Component%20Object%20Reference) (OtherActor :type Actor%20Object%20Reference) (OtherComp :type Primitive%20Component%20Object%20Reference) (OtherBodyIndex :type Integer) (bFromSweep :type Boolean) (SweepResult :type Hit%20Result%20Structure%20%28by%20ref%29))
  (bind _asbp_character (Utilities|Casting|CastToBP_Character OtherActor))
  (if (Pawn|IsLocallyControlled _asbp_character)
    (bind _asplayer_controller (Utilities|Casting|CastToPlayerController (Pawn|GetController _asbp_character)))
    (Input|EnableInput _asplayer_controller)
    (Variables|Default|SetTecla%20C true)))

(event OnComponentEndOverlap(Sphere)
  (params (OverlappedComponent :type Primitive%20Component%20Object%20Reference) (OtherActor :type Actor%20Object%20Reference) (OtherComp :type Primitive%20Component%20Object%20Reference) (OtherBodyIndex :type Integer))
  (bind _asbp_character (Utilities|Casting|CastToBP_Character OtherActor))
  (if (Pawn|IsLocallyControlled _asbp_character)
    (bind _asplayer_controller (Utilities|Casting|CastToPlayerController (Pawn|GetController _asbp_character)))
    (Input|DisableInput _asplayer_controller)
    (Variables|Default|SetTecla%20C false)))

(event EventBeginPlay)

(event Collision|EventActorBeginOverlap
  (params (OtherActor :type Actor%20Object%20Reference)))

(event EventTick
  (params (DeltaSeconds :type Float%20%28single-precision%29)))

(event Input|KeyboardEvents|C
  (params (Key :type Key%20Structure :default "None"))
  (:Pressed
    (Utilities|FlowControl|FlipFlop
      (:A
        (if (Variables|Default|GetTecla%20C)
          (Default|ServerGuardarProgreso (stale OnComponentBeginOverlap(Sphere) _asbp_character))
          (bind _returnvalue (UserInterface|CreateWidget "/Game/ui/WBP_Crafteo.WBP_Crafteo_C"))
          (UserInterface|Viewport|AddtoViewport _returnvalue 0)
          (bind _output_get (Variables|Default|SetWBP _returnvalue))
          (Input|SetInputModeGameandUI (Game|GetPlayerController (Variables|/Script/Engine.Pawn|GetPlayerState (stale OnComponentBeginOverlap(Sphere) _asbp_character))) _output_get "DoNotLock" true false)
          (Variables|/Script/Engine.PlayerController|SetbShowMouseCursor (stale OnComponentBeginOverlap(Sphere) _asplayer_controller) true)))
      (:B
        (if (Variables|Default|GetTecla%20C)
          (Widget|RemovefromParent (Variables|Default|GetWBP))
          (Input|SetInputModeGameOnly (stale OnComponentBeginOverlap(Sphere) _asplayer_controller) false)
          (Variables|/Script/Engine.PlayerController|SetbShowMouseCursor (stale OnComponentBeginOverlap(Sphere) _asplayer_controller) false))))))

(fn ConstructionScript)