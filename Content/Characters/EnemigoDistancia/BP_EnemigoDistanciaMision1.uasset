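; Mission 1 ranged nun enemy that targets the player with projectile and melee attacks.
; Ranged attacks play a multicast shoot montage and spawn BP_Proyectil at the target; melee plays a multicast montage and sphere-traces at the weapon socket, damaging through an interface.
; Health events update a widget progress bar.
; Local damage, death, objective, XP and potion-drop chains are disconnected and never run.
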(event OnComponentHit(CapsuleComponent)
  (params (HitComponent :type Primitive%20Component%20Object%20Reference) (OtherActor :type Actor%20Object%20Reference) (OtherComp :type Primitive%20Component%20Object%20Reference) (NormalImpulse :type Vector :default "0, 0, 0") (Hit :type Hit%20Result%20Structure%20%28by%20ref%29)))

(event Custom|Multicast_PlayAtaqueMele
  (Animation|Montage|PlayMontage (Variables|Character|GetMesh) "/Game/Characters/EnemigoDistancia/NewFolder/ENEMIGO_DISTANCIA_MONJA_Anim_Anim_Enemy_Monja_Atack_v2_Montage1.ENEMIGO_DISTANCIA_MONJA_Anim_Anim_Enemy_Monja_Atack_v2_Montage1"
    (:then
      _)
    (:OnNotifyBegin
      _))
  (Variables|Default|SetEstaatacando true)
  (Utilities|FlowControl|Delay 1.0))

(event Custom|Multicast_PlayAnimacionDisparo
  (Animation|Montage|PlayMontage (Variables|Character|GetMesh) "/Game/Characters/EnemigoDistancia/NewFolder/ENEMIGO_DISTANCIA_MONJA_Anim_Anim_Enemy_Monja_Shoot_v2_Montage.ENEMIGO_DISTANCIA_MONJA_Anim_Anim_Enemy_Monja_Shoot_v2_Montage"
    (:then
      _)
    (:OnInterrupted
      _)
    (:OnNotifyBegin
      _))
  (Variables|Default|SetEstaDisparando_0 true)
  (Utilities|FlowControl|Delay 0.8))

(event EventBeginPlay
  (|CallParentFunction)
  (CallFunction|SetTarget (CallFunction|GetMyPlayerCharacter))
  (Variables|Default|SetAnimacionmuerte "/Game/Characters/EnemigoDistancia/NewFolder/ENEMIGO_DISTANCIA_MONJA_Anim_Anim_Enemy_Monja_Death_v2_Montage.ENEMIGO_DISTANCIA_MONJA_Anim_Anim_Enemy_Monja_Death_v2_Montage"))

(event Collision|EventActorBeginOverlap
  (params (OtherActor :type Actor%20Object%20Reference))
  (|CallParentFunction OtherActor) ; This node is disabled and will not be called.\nDrag off pins to build functionality.
)

(event EventTick
  (params (DeltaSeconds :type Float%20%28single-precision%29))
  (|CallParentFunction DeltaSeconds))

(event EventSaludInicialEnemigo
  (params (Vida :type Float%20%28double-precision%29) (Vida%20max :type Float%20%28double-precision%29))
  (bind _aswbp_barra_vida_enemigo (Utilities|Casting|CastToWBP_BarraVidaEnemigo (UserInterface|GetWidget (Variables|Default|GetWidget))))
  (Variables|Default|SetAs%20WBP%20Barra%20Vida%20Enemigo_0 _aswbp_barra_vida_enemigo)
  (CallFunction|ActualizarVidaInicialMonja Vida Vida%20max))

(event EventAtaqueMonja
  (CallFunction|MulticastPlayAtaqueMele)
  (CallFunction|HitDetect)
  (Variables|Default|SetEstaatacando false))

(event EventEnemigoRecibioDano
  (params (Vida :type Float%20%28double-precision%29) (Vida%20max :type Float%20%28double-precision%29))
  (CallFunction|ActualizarVidaInicialMonja Vida Vida%20max))

(event EventAtaqueDistancia
  (CallFunction|MulticastPlayAnimacionDisparo)
  (CallFunction|DisparoMonja (Variables|Default|GetTarget))
  (Variables|Default|SetEstaDisparando_0 false))

(fn ConstructionScript
  (|CallParentFunction))

(fn DisparoMonja
  (params (objetivo :type BP%20Character%20Object%20Reference))
  (Variables|Default|SetTarget objetivo)
  (Game|SpawnActorfromClass "/Game/Characters/EnemigoDistancia/BP_Proyectil.BP_Proyectil_C" (Transformation|GetActorTransform) "AlwaysSpawn" "MultiplyWithRoot" 0 1e+01 (Variables|Default|GetDaño%20Proyectil_0) (Variables|Default|GetTarget) 0))

(fn ActualizarVidaInicialMonja
  (params (vida :type Float%20%28double-precision%29) (Vida%20Max :type Float%20%28double-precision%29))
  (bind _as_wbp_barra_vida_enemigo_0 (Variables|Default|GetAs%20WBP%20Barra%20Vida%20Enemigo_0))
  (bind _progressbar_vidaenemigo (Variables|/Game/ui/BarraVidaEnemigo/WBP_BarraVidaEnemigo.WBP_BarraVidaEnemigo_C|GetProgressBar_vidaenemigo _as_wbp_barra_vida_enemigo_0))
  (Utilities|IsValid _progressbar_vidaenemigo
    (:Is%20Valid
      (Progress|SetPercent _progressbar_vidaenemigo (/ vida Vida%20Max)))))

(fn SetTarget
  (params (Target :type BP%20Character%20Object%20Reference))
  (Variables|Default|SetTarget Target))

(fn HitDetect
  (bind _mesh (Variables|Character|GetMesh))
  (bind _returnvalue (Transformation|GetSocketLocation _mesh "MonjaArmaSocket"))
  (bind _outhit (Collision|SphereTraceForObjects _returnvalue _returnvalue 3e+01 (Utilities|Array|MakeArray "ObjectTypeQuery7") false 0 "ForDuration"))
  (if (Utilities|DoesObjectImplementInterface (.HitActor (Collision|BreakHitResult _outhit)) "/Script/proyectoejercicio.interfazparahacerdanio")
    (Class|Interfazparahacerdanio|RealizarDanio(Message) (.HitActor (Collision|BreakHitResult _outhit)) (Variables|Default|GetDañoMele))))