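; Boss character Jefe Congregacion, with a melee attack and an arena health bar.
; AtaqueMonja calls MulticastDanioMele for the montage and delayed Niagara effect, then immediately sphere-traces below the attack socket, applying damage through an interface.
; BeginPlay targets the player character, and GolpeVampiro forwards incoming damage to RecibirDanioInterfaz.
; The arena trigger shows the boss's health once on the locally controlled player's HUD.
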(event OnComponentBeginOverlap(TriggerArena)
  (params (OverlappedComponent :type Primitive%20Component%20Object%20Reference) (OtherActor :type Actor%20Object%20Reference) (OtherComp :type Primitive%20Component%20Object%20Reference) (OtherBodyIndex :type Integer) (bFromSweep :type Boolean) (SweepResult :type Hit%20Result%20Structure%20%28by%20ref%29))
  (bind _asbp_character (Utilities|Casting|CastToBP_Character OtherActor))
  (if (Pawn|IsLocallyControlled _asbp_character)
    (bind _asbp_player_controller_nuevo (Utilities|Casting|CastToBP_PlayerControllerNuevo (Pawn|GetController _asbp_character)))
    (Utilities|FlowControl|DoOnce false
      (:Completed
        (Default|MostrarVidaBoss (Variables|/Game/BP_PlayerControllerNuevo.BP_PlayerControllerNuevo_C|GetRef_HUD_Principal _asbp_player_controller_nuevo) self)))))

(event Custom|MulticastDanioMele
  (Animation|Montage|PlayMontage (Variables|Character|GetMesh) "/Game/Characters/JefeCongregacion/Animaciones/BossJefeCongregacion_Anim_Rig_BossJefeCongregacion_anim_BossJefeCongregacion_Atack_Montage.BossJefeCongregacion_Anim_Rig_BossJefeCongregacion_anim_BossJefeCongregacion_Atack_Montage"
    (:then
      _)
    (:OnNotifyBegin
      _))
  (Variables|Default|SetEstaatacando true)
  (Utilities|FlowControl|Delay 1.0)
  (Niagara|SpawnSystematLocation "/Game/Characters/JefeCongregacion/NS_Mele.NS_Mele" (Transformation|GetSocketLocation (Variables|Character|GetMesh) "danioataquemele") (Transformation|GetActorRotation)))

(event EventBeginPlay
  (CallFunction|SetTarget (CallFunction|GetMyPlayerCharacter)))

(event Collision|EventActorBeginOverlap
  (params (OtherActor :type Actor%20Object%20Reference)))

(event EventTick
  (params (DeltaSeconds :type Float%20%28single-precision%29)))

(event EventAtaqueMonja
  (CallFunction|MulticastDanioMele)
  (CallFunction|HitDetect)
  (Variables|Default|SetEstaatacando false))

(event EventGolpeVampiro
  (params (daño :type Float%20%28double-precision%29) (Atacante :type BP%20Character%20Object%20Reference))
  (Class|MiniBoss|RecibirDanioInterfaz daño))

(fn ConstructionScript)

(fn HitDetect
  (bind _mesh (Variables|Character|GetMesh))
  (bind _returnvalue (Transformation|GetSocketLocation _mesh "danioataquemele"))
  (bind _outhit (Collision|SphereTraceForObjects _returnvalue (- _returnvalue "0.000000,0.000000,80.000000") 8e+01 (Utilities|Array|MakeArray "ObjectTypeQuery7") false 0 "ForDuration"))
  (if (Utilities|DoesObjectImplementInterface (.HitActor (Collision|BreakHitResult _outhit)) "/Script/proyectoejercicio.interfazparahacerdanio")
    (Class|Interfazparahacerdanio|RealizarDanio(Message) (.HitActor (Collision|BreakHitResult _outhit)) (Variables|Default|GetDanio))))

(fn SetTarget
  (params (Taget :type BP%20Character%20Object%20Reference))
  (Variables|Default|SetTaget Taget))