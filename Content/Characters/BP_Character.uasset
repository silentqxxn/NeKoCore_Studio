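; Networked player character handling melee and ranged combat, reloading from inventory, quest interactions, death and respawn at the start transform.
; CompExperiencia level-ups apply DT_DataProgreso multipliers through CompEstadisticas, while CompArmas supplies weapons and ammo.
; Server events handle shots, reloads and object quest progress, with client events updating the ammo HUD.
; Older BPComponenteVida still serves potions and AnyDamage; dash, look, save-loading and older respawn logic sit disconnected.
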(event OnPersonajeRevive(CompEstadisticas)
  (Variables|Default|SetEstaAtacando false))

(event Custom|Server_ProcesarInteraccion
  (params (ID_Objetivo :type Name))
  ;[0.15 0.15 0.15 0.5] Interactuar
  (bind _asbp_player_state_countless_blood (Utilities|Casting|CastToBP_PlayerStateCountlessBlood (Variables|Default|GetPlayerState))
    (:then
      (Class|ComponenteMisiones|ProgressObjective (Variables|/Script/proyectoejercicio.PlayerStateCountlessBlood|GetComponenteMisiones _asbp_player_state_countless_blood) ID_Objetivo "Interactuar" 1)
      (Development|PrintString "EXITO: SERVER PROCESO EL PUNTO\""))
    (:CastFailed
      (Development|PrintString "falla no hay player state"))))

(event Custom|Dano%20recibido
  (params (Vida :type Float%20%28double-precision%29) (Vida%20max :type Float%20%28double-precision%29))
  (Default|Actualizarvida (Variables|Default|Getui) Vida Vida%20max))

(event Custom|Server_UsarPocion
  (params (CuantoCura :type Float%20%28double-precision%29))
  ;[0.15 0.15 0.15 0.5] Vida
  (Default|RecibirCuracion (Variables|Default|GetBP_ComponenteVida) CuantoCura))

(event Custom|Server_GuardarProgreso
  (bind _returnvalue (SaveGame|CreateSaveGameObject "/Game/save/SG_SaveData.SG_SaveData_C"))
  (Default|SavePlayerData _returnvalue self)
  (SaveGame|SaveGametoSlot _returnvalue "PlayerData"))

(event Custom|salud%20inicial
  (params (Vida :type Float%20%28double-precision%29) (Vida%20max :type Float%20%28double-precision%29))
  (Default|Actualizarvida (Variables|Default|Getui) Vida Vida%20max))

(event Custom|SecuenciaMuerte
  (bind _respaw (Variables|Default|GetRespaw))
  (Utilities|FlowControl|Sequence
    (:then_0
      (Utilities|Casting|CastToPlayerControllerNuevo (Pawn|GetController))
      (Input|DisableInput 0)
      (Animation|PlayAnimMontage "/Game/Characters/Chrt_Condesa/Animaciones/muerte/ANIM_CONDESA_Anim_Anim_death_001_Montage.ANIM_CONDESA_Anim_Anim_death_001_Montage" 1.0 "None"))
    (:then_1
      (Input|DisableInput 0)
      (Animation|PlayAnimMontage "/Game/Characters/Chrt_Condesa/Animaciones/muerte/ANIM_CONDESA_Anim_Anim_death_001_Montage.ANIM_CONDESA_Anim_Anim_death_001_Montage" 1.0 "None")
      (Utilities|FlowControl|Delay 2.0)
      (Transformation|Teleport (.location _respaw) (.rotation _respaw))
      (Networking|SwitchHasAuthority
        (:Authority
          (Class|ComponenteEstadisticas|ServerRevivir (Variables|Default|GetCompEstadisticas)))
        (:Remote
          _))
      (Input|EnableInput 0))))

(event Custom|MulticastMuerte)

(event Custom|RPC_Server_Ataque
  ;[0.15 0.15 0.15 0.5] ataque mele
  (CallFunction|RPCAttackcliente))

(event Custom|RPC_SpawndeArmas
  (params (spawnarma :type BP%20Armas%20Master%20Attach%20Class%20Reference))
  ;[0.15 0.15 0.15 0.5] Sistema de armas
)

(event Custom|Cliente_MostrarMisionCompletada)

(event Custom|IniciarRespawn)

(event Custom|RPC_attackcliente
  ;[0.15 0.15 0.15 0.5] ataque mele
  (if (not (Variables|Default|GetDashAcrtivado?))
    (if (not (AI|Components|NavMovement|IsFalling (Variables|Character|GetCharacterMovement)))
      (if (not (Variables|Default|GetEstaAtacando))
        (Pawn|Components|CharacterMovement|DisableMovement (Variables|Character|GetCharacterMovement))
        (Variables|Default|SetEstaAtacando true)
        (Animation|Montage|PlayMontage (Variables|Character|GetMesh) "/Game/Characters/Chrt_Condesa/Animaciones/Ataque/CHRT_CONDESA_V9_Anim_Anim_Atack_Montage.CHRT_CONDESA_V9_Anim_Anim_Atack_Montage"
          (:then
            (CallFunction|HitDetect)
            (Utilities|FlowControl|Delay 0.5)
            (Pawn|Components|CharacterMovement|SetMovementMode (Variables|Character|GetCharacterMovement) "MOVE_Walking" 0))
          (:OnCompleted
            (Variables|Default|SetEstaAtacando false)
            (Variables|Default|SetPuede_Daño true)))))))

(event Custom|Dis)

(event Custom|Cliente_MostrarContador)

(event Custom|Server_Respawn)

(event Custom|Client_Despertar
  (bind _asbp_player_controller_nuevo (Utilities|Casting|CastToBP_PlayerControllerNuevo (Pawn|GetController)))
  (Input|EnableInput _asbp_player_controller_nuevo))

(event Custom|MC_CaerMuerto
  (if (Pawn|IsLocallyControlled)
    (Input|DisableInput (Game|GetPlayerController 0))))

(event Custom|ServerSpawnProyectil
  (params (DireccionDisparo :type Rotator))
  (bind _returnvalue (Transformation|GetActorLocation))
  (bind _comparmas (Variables|Default|GetCompArmas))
  (bind _comparmas_2 (Variables|Default|GetCompArmas))
  (bind _compestadisticas (Variables|Default|GetCompEstadisticas))
  (bind _armaespalda (Variables|/Script/proyectoejercicio.ComponenteArmas|GetArmaEspalda _comparmas))
  (bind _armaespalda_2 (Variables|/Script/proyectoejercicio.ComponenteArmas|GetArmaEspalda _comparmas_2))
  (bind _ataqueactual (Variables|/Script/proyectoejercicio.ComponenteEstadisticas|GetAtaqueActual _compestadisticas))
  (bind _damage (Variables|/Script/proyectoejercicio.WeaponMaster|GetDamage _armaespalda_2))
  (bind _returnvalue_2 (+ _ataqueactual _damage))
  ;[0.15 0.15 0.15 0.5] ataque distancia
  (if (not (Variables|Default|GetDashAcrtivado?))
    (if (not (Variables|Default|GetEstaAtacando))
      (if (> (Variables|/Script/proyectoejercicio.WeaponMaster|GetMunicionActual _armaespalda) 0)
        (bind _output_get (Variables|/Script/proyectoejercicio.WeaponMaster|SetMunicionActual _armaespalda (- (Variables|/Script/proyectoejercicio.WeaponMaster|GetMunicionActual _armaespalda) 1)))
        (CallFunction|ClientActualizarUIMunicion self _output_get (Variables|/Script/proyectoejercicio.WeaponMaster|GetCapacidadCargador _armaespalda))
        (Collision|LineTraceForObjects _returnvalue (+ _returnvalue (* (Math|Vector|GetForwardVector DireccionDisparo) (Variables|Default|GetAlcanceDisparo))) (Utilities|Array|MakeArray "ObjectTypeQuery1" "ObjectTypeQuery2" "ObjectTypeQuery8") false 0 "None")
        (Pawn|Components|CharacterMovement|DisableMovement (Variables|Character|GetCharacterMovement))
        (Game|SpawnActorfromClass "/Game/quest/actores/BP_ProyectilDistancia.BP_ProyectilDistancia_C" (Transformation|GetWorldTransform (Variables|Default|GetArrow1)) "AdjustIfPossibleButAlwaysSpawn" "MultiplyWithRoot" 0 _returnvalue_2 self self)
        (Utilities|FlowControl|Delay 0.5)
        (Pawn|Components|CharacterMovement|SetMovementMode (Variables|Character|GetCharacterMovement) "MOVE_Walking" 0)
        (Development|PrintString (Utilities|String|ToString(Float) _returnvalue_2))))))

(event Custom|Server_RecargarArma
  (bind _comparmas (Variables|Default|GetCompArmas))
  (bind _compinventario (Variables|Default|GetCompInventario))
  (bind (_outitem _returnvalue) (Class|ComponenteInventario|QueryInventory _compinventario "BalasDePlata"))
  (bind _armaespalda (Variables|/Script/proyectoejercicio.ComponenteArmas|GetArmaEspalda _comparmas))
  (bind _capacidadcargador (Variables|/Script/proyectoejercicio.WeaponMaster|GetCapacidadCargador _armaespalda))
  ;[0.15 0.15 0.15 0.5] Recarga
  (if (< (Variables|/Script/proyectoejercicio.WeaponMaster|GetMunicionActual _armaespalda) 5)
    (if _returnvalue
      (Class|ComponenteInventario|ServerQuitarItem (Variables|Default|GetCompInventario) "BalasDePlata" (Math|Integer|Min(Integer) (- _capacidadcargador (Variables|/Script/proyectoejercicio.WeaponMaster|GetMunicionActual _armaespalda)) (.Cantidad (Utilities|Struct|BreakItemData _outitem))))
      (bind _output_get (Variables|/Script/proyectoejercicio.WeaponMaster|SetMunicionActual (Variables|/Script/proyectoejercicio.ComponenteArmas|GetArmaEspalda (Variables|Default|GetCompArmas)) (+ (Math|Integer|Min(Integer) (- _capacidadcargador (Variables|/Script/proyectoejercicio.WeaponMaster|GetMunicionActual _armaespalda)) (.Cantidad (Utilities|Struct|BreakItemData _outitem))) (Variables|/Script/proyectoejercicio.WeaponMaster|GetMunicionActual _armaespalda))))
      (CallFunction|ClientActualizarUIMunicion self _output_get _capacidadcargador))))

(event Custom|Client_ActualizarUIMunicion
  (params (BalasActuales :type Integer) (BalasMaximas :type Integer))
  ;[0.15 0.15 0.15 0.5] Actualizar municion
  (bind _asbp_player_controller_nuevo (Utilities|Casting|CastToBP_PlayerControllerNuevo (Pawn|GetController)))
  (Utilities|IsValid (Variables|/Game/BP_PlayerControllerNuevo.BP_PlayerControllerNuevo_C|GetRef_HUD_Principal _asbp_player_controller_nuevo)
    (:Is%20Valid
      (Default|ActualizarTextosMunicion (Variables|/Game/ui/WBP_ui.WBP_ui_C|GetWBP_MunicionInterno (Variables|/Game/BP_PlayerControllerNuevo.BP_PlayerControllerNuevo_C|GetRef_HUD_Principal _asbp_player_controller_nuevo)) BalasActuales BalasMaximas))))

(event Custom|SumoExperiencia
  (params (XP :type Float%20%28double-precision%29) (XP%20Max :type Float%20%28double-precision%29))
  (Default|ActualizarEXP (Variables|Default|Getui) XP XP%20Max))

(event Custom|SumoLevel
  (params (nivel :type Integer))
  (Default|ActualizarLVL (Variables|Default|Getui) nivel))

(event Custom|CuracionRecibida
  (params (Vida :type Float%20%28double-precision%29) (VidaMax :type Float%20%28double-precision%29))
  (Default|Actualizarvida (Variables|Default|Getui) Vida VidaMax))

(event Custom|ExperienciaAlEmpezar
  (params (XP :type Float%20%28double-precision%29) (XPMax :type Float%20%28double-precision%29))
  (Default|ActualizarEXP (Variables|Default|Getui) XP XPMax))

(event Custom|levelinicial
  (params (level :type Integer))
  (Default|ActualizarLVL (Variables|Default|Getui) level))

(event Custom|AplicarMejorasNivel
  (params (NivelAnterior :type Integer) (NivelNuevo :type Integer))
  (bind _returnvalue (Utilities|GetDataTableRow "/Game/Datatable/DT_DataProgreso.DT_DataProgreso" (Utilities|String|StringToName (Utilities|String|ToString(Integer) NivelNuevo)))
    (:then
      (Class|ComponenteEstadisticas|ServerAplicarMultiplicadoresNivel (Variables|Default|GetCompEstadisticas) (.PorcentajeHP (Utilities|Struct|BreakProgresoNivelRow _returnvalue)) (.PorcentajeAtaque (Utilities|Struct|BreakProgresoNivelRow _returnvalue)) (.PorcentajeVelocidad (Utilities|Struct|BreakProgresoNivelRow _returnvalue)) (.PorcentajeDefensa (Utilities|Struct|BreakProgresoNivelRow _returnvalue))))))

(event Custom|DashCompletado
  ;[0.15 0.15 0.15 0.5] dash
  (Variables|/Script/Engine.CharacterMovementComponent|SetGravityScale (Variables|Character|GetCharacterMovement) 1.0)
  (Collision|SetCollisionEnabled (Variables|Default|GetCapsuleComponent) "QueryAndPhysics")
  (Utilities|Time|ClearTimerbyFunctionName 0 "DashCompletado"))

(event Input|EnhancedActionEvents|EnhancedInputActionIA_Stats
  (params (ActionValue :type Boolean) (ElapsedSeconds :type Float%20%28double-precision%29) (TriggeredSeconds :type Float%20%28double-precision%29) (InputAction :type Input%20Action%20Object%20Reference :default "/Game/imputs/IA_Stats.IA_Stats"))
  (bind _ref_widgetstats (Variables|Default|GetREF_WidgetStats))
  ;[0.15 0.15 0.15 0.5] Manu Stats
  (:Started
    (if (Variables|Default|GetMenu%20stats%20abierto?)
      (Widget|SetVisibility _ref_widgetstats "Hidden")
      (Variables|Default|SetMenu%20stats%20abierto? false)
      (else
        (Widget|SetVisibility _ref_widgetstats "Visible")
        (Variables|Default|SetMenu%20stats%20abierto? true)))))

(event Input|EnhancedActionEvents|EnhancedInputActionIA_Dash
  (params (ActionValue :type Boolean) (ElapsedSeconds :type Float%20%28double-precision%29) (TriggeredSeconds :type Float%20%28double-precision%29) (InputAction :type Input%20Action%20Object%20Reference :default "/Game/imputs/IA_Dash.IA_Dash"))
  ;[0.15 0.15 0.15 0.5] dash
)

(event Input|EnhancedActionEvents|EnhancedInputActionIA_Mirar
  (params (ActionValue :type Vector%202D%20Structure) (ElapsedSeconds :type Float%20%28double-precision%29) (TriggeredSeconds :type Float%20%28double-precision%29) (InputAction :type Input%20Action%20Object%20Reference :default "/Game/imputs/IA_Mirar.IA_Mirar")))

(event Input|EnhancedActionEvents|EnhancedInputActionIA_AtaqueMele
  (params (ActionValue :type Boolean) (ElapsedSeconds :type Float%20%28double-precision%29) (TriggeredSeconds :type Float%20%28double-precision%29) (InputAction :type Input%20Action%20Object%20Reference :default "/Game/imputs/IA_AtaqueMele.IA_AtaqueMele"))
  ;[0.15 0.15 0.15 0.5] ataque mele
  (:Started
    (Utilities|IsValid (Variables|/Script/proyectoejercicio.ComponenteArmas|GetArmaManoDerecha (Variables|Default|GetCompArmas))
      (:Is%20Valid
        (CallFunction|RPCServerAtaque)))))

(event Input|EnhancedActionEvents|EnhancedInputActionIA_Recargar
  (params (ActionValue :type Boolean) (ElapsedSeconds :type Float%20%28double-precision%29) (TriggeredSeconds :type Float%20%28double-precision%29) (InputAction :type Input%20Action%20Object%20Reference :default "/Game/imputs/IA_Recargar.IA_Recargar"))
  ;[0.15 0.15 0.15 0.5] Recarga
  (:Started
    (CallFunction|ServerRecargarArma)))

(event Input|EnhancedActionEvents|EnhancedInputActionIA_Interactuar
  (params (ActionValue :type Boolean) (ElapsedSeconds :type Float%20%28double-precision%29) (TriggeredSeconds :type Float%20%28double-precision%29) (InputAction :type Input%20Action%20Object%20Reference :default "/Game/imputs/IA_Interactuar.IA_Interactuar"))
  ;[0.15 0.15 0.15 0.5] Interactuar
  (CallFunction|InteractTrace)
  (bind _lookatactor (Variables|Default|GetLookAtActor)
    (:then
      (bind (_objetiveid _esnpc_) (Class|BPIInteractionQuest|Interactwith(Message) _lookatactor))
      (if _esnpc_
        (bind _asbp_quest_base (Utilities|Casting|CastToBP_QuestBase _lookatactor))
        (Default|OnObjetiveIDHeard _asbp_quest_base _objetiveid 1)
        (else
          (CallFunction|ServerProcesarInteraccion _objetiveid))))
    (:else)))

(event Input|EnhancedActionEvents|EnhancedInputActionIA_Menu
  (params (ActionValue :type Boolean) (ElapsedSeconds :type Float%20%28double-precision%29) (TriggeredSeconds :type Float%20%28double-precision%29) (InputAction :type Input%20Action%20Object%20Reference :default "/Game/imputs/IA_Menu.IA_Menu")))

(event Game|Damage|EventAnyDamage
  (params (Damage :type Float%20%28single-precision%29) (DamageType :type Damage%20Type%20Object%20Reference) (InstigatedBy :type Controller%20Object%20Reference) (DamageCauser :type Actor%20Object%20Reference))
  ;[0.15 0.15 0.15 0.5] Vida
  (Default|DañoAlJugar (Variables|Default|GetBP_ComponenteVida) Damage))

(event Collision|EventActorBeginOverlap
  (params (OtherActor :type Actor%20Object%20Reference)))

(event EventTick
  (params (DeltaSeconds :type Float%20%28single-precision%29)))

(event EventDanoesfera
  (params (dano :type Float%20%28double-precision%29))
  ;[0.15 0.15 0.15 0.5] Recibir Daño
  (if (Ability|HasAuthority)
    (Class|ComponenteEstadisticas|ServerRecibirDanio (Variables|Default|GetCompEstadisticas) dano)))

(event EventRealizarDanio
  (params (danio :type Float%20%28single-precision%29))
  ;[0.15 0.15 0.15 0.5] Recibir Daño
  (if (Ability|HasAuthority)
    (Class|ComponenteEstadisticas|ServerRecibirDanio (Variables|Default|GetCompEstadisticas) danio)))

(event EventObtenerExperiencia
  (params (Experiencia :type Integer))
  ;[0.15 0.15 0.15 0.5] Experiencia
  (Class|ComponenteExperiencia|ServerAgregarXP (Variables|Default|GetCompExperiencia) Experiencia))

(event EventEjecutarDisparoRanged
  (params (Direccion :type Rotator :default "0, 0, 0"))
  ;[0.15 0.15 0.15 0.5] ataque distancia
  (CallFunction|ServerSpawnProyectil Direccion))

(event EventBeginPlay
  (bind _compexperiencia (Variables|Default|GetCompExperiencia))
  (EventDispatchers|BindEventtoOnSubeNivel _compexperiencia (delegate Custom|AplicarMejorasNivel))
  (CallFunction|AplicarMejorasNivel 0 (Class|ComponenteExperiencia|GetNivel _compexperiencia))
  (bind _returnvalue (UserInterface|CreateWidget "/Game/ui/stats/WBP_Estadisticas.WBP_Estadisticas_C"))
  (bind _output_get (Variables|Default|SetREF_WidgetStats _returnvalue))
  (UserInterface|Viewport|AddtoViewport _output_get 0)
  (Widget|SetVisibility (Variables|Default|GetREF_WidgetStats) "Hidden")
  (EventDispatchers|BindEventtoOnPersonajeMuere (Variables|Default|GetCompEstadisticas) (delegate Custom|SecuenciaMuerte))
  (Variables|Default|SetRespaw (Transformation|GetActorTransform)))

(event Input|KeyboardEvents|DebugKeyM
  (params (Key :type Key%20Structure :default "None") (ActionValue :type Input%20Action%20Value%20Structure))
  (bind _returnvalue (Game|GetPlayerController 0))
  ;[0.15 0.15 0.15 0.5] menu pausa debug
  (:Pressed
    (if (Utilities|IsValid (Variables|Default|GetPausaRef))
      (Development|PrintString "true")
      (Widget|RemovefromParent (Variables|Default|GetPausaRef))
      (Game|SetGamePaused true)
      (Variables|/Script/Engine.PlayerController|SetbShowMouseCursor _returnvalue false)
      (Variables|Default|SetPausaRef 0)
      (else
        (Development|PrintString "false")
        (bind _returnvalue_2 (UserInterface|CreateWidget "/Game/ui/WBP_MenuPausa.WBP_MenuPausa_C"))
        (bind _output_get (Variables|Default|SetPausaRef _returnvalue_2))
        (UserInterface|Viewport|AddtoViewport _output_get 0)
        (Game|SetGamePaused true)
        (Variables|/Script/Engine.PlayerController|SetbShowMouseCursor _returnvalue true)
        (Variables|Default|SetJuegoPausado? true)))))

(event Input|KeyboardEvents|DebugKeyP
  (params (Key :type Key%20Structure :default "None") (ActionValue :type Input%20Action%20Value%20Structure)))

(event Input|KeyboardEvents|DebugKey1
  (params (Key :type Key%20Structure :default "None") (ActionValue :type Input%20Action%20Value%20Structure))
  ;[0.15 0.15 0.15 0.5] Vida
  (:Pressed
    (if (> (Variables|Default|GetContador%20de%20Pociones_Comunes) 0)
      (CallFunction|ServerUsarPocion 25.0))))

(fn ConstructionScript)

(fn ActualizarUi
  (bind _bp_componentevida (Variables|Default|GetBP_ComponenteVida))
  (bind _asbp_player_controller_nuevo (Utilities|Casting|CastToBP_PlayerControllerNuevo (Pawn|GetController)))
  (Utilities|IsValid (Variables|/Game/BP_PlayerControllerNuevo.BP_PlayerControllerNuevo_C|GetRef_HUD_Principal _asbp_player_controller_nuevo)
    (:Is%20Valid
      (Progress|SetPercent (Variables|/Game/ui/WBP_ui.WBP_ui_C|GetProgressBar_vida (Variables|/Game/BP_PlayerControllerNuevo.BP_PlayerControllerNuevo_C|GetRef_HUD_Principal _asbp_player_controller_nuevo)) (/ (Variables|/Game/componente/BP_ComponenteVida.BP_ComponenteVida_C|GetVida _bp_componentevida) (Variables|/Game/componente/BP_ComponenteVida.BP_ComponenteVida_C|GetVida%20max _bp_componentevida))))))

(fn HitDetect
  (bind _mesh (Variables|Character|GetMesh))
  (bind _returnvalue (Transformation|GetSocketLocation _mesh "DanoArma"))
  (bind _outhit (Collision|SphereTraceForObjects _returnvalue _returnvalue 3e+01 (Utilities|Array|MakeArray "ObjectTypeQuery8") false 0 "ForDuration"))
  (if (Utilities|DoesObjectImplementInterface (.HitActor (Collision|BreakHitResult _outhit)) "/Game/interfase/BPI_AtaqueMele.BPI_AtaqueMele_C")
    (Class|BPIAtaqueMele|GolpeVampiro(Message) (.HitActor (Collision|BreakHitResult _outhit)) 33.0 self)))

(fn InteractTrace
  (bind _returnvalue (Transformation|GetActorLocation))
  (bind (_outhit _returnvalue_2) (Collision|SphereTraceForObjects _returnvalue _returnvalue 1e+02 (Utilities|Array|MakeArray "ObjectTypeQuery3") false 0 "Persistent"))
  (if _returnvalue_2
    (if (Utilities|DoesObjectImplementInterface (.HitActor (Collision|BreakHitResult _outhit)) "/Game/interfase/BPI_InteractionQuest.BPI_InteractionQuest_C")
      (bind _output_get (Variables|Default|SetLookAtActor (.HitActor (Collision|BreakHitResult _outhit))))
      (Class|BPIInteractionQuest|Lookat(Message) _output_get)
      (else
        (Variables|Default|SetLookAtActor 0)))
    (else
      (Variables|Default|SetLookAtActor 0))))

(fn OnRepVida)

(fn OnRepVidaMax)

(fn CalcularEstadisticasServidor)