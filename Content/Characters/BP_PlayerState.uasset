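; Player state Blueprint that tracks a blood-based leveling progression, holding current blood, current level and the threshold for the next level.
; AñadirSangreSrv adds blood and, on reaching the threshold, raises the level, carries the surplus over and multiplies the next threshold by a fixed growth factor.
; The threshold is checked once per call, so a large gain grants only one level at a time.
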(event EventBeginPlay)

(event EventTick
  (params (DeltaSeconds :type Float%20%28single-precision%29)))

(fn ConstructionScript)

(fn AñadirSangreSrv
  (params (Cantidad :type Float%20%28double-precision%29))
  (Variables|Default|SetSangreActual (+ (Variables|Default|GetSangreActual) Cantidad))
  (if (>= (Variables|Default|GetSangreActual) (Variables|Default|GetangreSiguienteNivel))
    (Variables|Default|SetNivelActual (+ (Variables|Default|GetNivelActual) 1))
    (Variables|Default|SetSangreActual (- (Variables|Default|GetSangreActual) (Variables|Default|GetangreSiguienteNivel)))
    (Variables|Default|SetangreSiguienteNivel (* (Variables|Default|GetangreSiguienteNivel) 1.5))))