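; Quest manager component that tracks active and completed quests by ID.
; Adding a quest spawns a BP_QuestBase actor and stores it for lookup by ID.
; Completing one moves its ID to the completed list and calls OnQuestCompleted with its actor, which stays in the array.
; Turn-in also sends the current stage's XP reward to the player character through an ObtenerExperiencia message; TrackQuest is an empty stub.
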(event EventBeginPlay)

(event EventTick
  (params (DeltaSeconds :type Float%20%28single-precision%29)))

(fn AddNewQuest
  (params (QuestID :type Name))
  (Utilities|Array|AddUnique (Variables|Default|GetCurrentActiveQuest) QuestID)
  (bind _returnvalue (Game|SpawnActorfromClass "/Game/quest/actores/BP_QuestBase.BP_QuestBase_C" (Math|Transform|MakeTransform "0, 0, 0" "0, 0, 0" "1.000000,1.000000,1.000000") "Undefined" "MultiplyWithRoot" 0 QuestID 0))
  (Utilities|Array|Add (Variables|Default|GetCurrentQuest) _returnvalue)
  (return _returnvalue))

(fn CompleteQuest
  (params (QuestID :type Name%20%28by%20ref%29))
  (Utilities|Array|AddUnique (Variables|Default|GetCompletedQuest) QuestID)
  (Utilities|Array|RemoveItem (Variables|Default|GetCurrentActiveQuest) QuestID)
  (bind _array_element (CallFunction|GetQuestActor QuestID))
  (Default|CallOnQuestCompleted _array_element))

(fn QueryActiveQuest
  (params (QuestID :type Name))
  (return (Utilities|Array|ContainsItem (Variables|Default|GetCurrentActiveQuest) QuestID)))

(fn TrackQuest)

(fn GetQuestActor
  (params (QuestID :type Name))
  (for _array_element (Variables|Default|GetCurrentQuest)
    (if (== (Variables|/Game/quest/actores/BP_QuestBase.BP_QuestBase_C|GetQuestID _array_element) QuestID)
      (return _array_element))))

(fn TurinQuest
  (params (QuestId :type Name))
  (Utilities|FlowControl|Sequence
    (:then_0
      (bind _array_element (CallFunction|GetQuestActor QuestId)))
    (:then_1
      (CallFunction|CompleteQuest QuestId)
      (Class|BPIExperiencia|ObtenerExperiencia(Message) (Game|GetPlayerCharacter 0) (.XPRewards (Utilities|Struct|BreakS_StageDetails (Variables|/Game/quest/actores/BP_QuestBase.BP_QuestBase_C|GetCurrentStageDetails _array_element)))))))