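; BP_ComponenteExperiencia is an experience component that tracks XP, the XP threshold and the player level.
; IncrementarExperiencia adds XP and loops IncrementarLevel while XP exceeds MaxXP, raising the threshold 25% per level and then subtracting that new threshold from XP.
; Event dispatchers broadcast XP and level changes, plus initial values one tick after BeginPlay.
; A debug print shows the values on each gain.
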(event EventBeginPlay
  (Utilities|FlowControl|DelayUntilNextTick)
  (CallFunction|ExpInicial)
  (CallFunction|LevelInicial))

(event EventTick
  (params (DeltaSeconds :type Float%20%28single-precision%29)))

(fn IncrementarExperiencia
  (params (XP%20Añadida :type Float%20%28double-precision%29))
  (bind _max_xp (Variables|Default|GetMax%20XP))
  (bind _max_xp_2 (Variables|Default|GetMax%20XP))
  (Variables|Default|SetXP (+ (Variables|Default|GetXP) XP%20Añadida))
  (while (> (Variables|Default|GetXP) _max_xp_2)
    (CallFunction|IncrementarLevel 1 (+ (Variables|Default|GetMax%20XP) (* _max_xp_2 0.25)))
    (Default|CallSuboExperiencia (Variables|Default|GetXP) _max_xp)
    (Development|PrintString (Utilities|String|Append "MAX EXP" (Utilities|String|ToString(Float) _max_xp) " 
XP" (Utilities|String|ToString(Float) (Variables|Default|GetXP)) " 
LEVEL" (Utilities|String|ToString(Integer) (Variables|Default|GetLevelPlayer))) true true "(R=0.000000,G=0.660000,B=1.000000,A=1.000000)" 1e+01))
  (Default|CallSuboExperiencia (Variables|Default|GetXP) _max_xp)
  (Development|PrintString (Utilities|String|Append "MAX EXP" (Utilities|String|ToString(Float) _max_xp) " 
XP" (Utilities|String|ToString(Float) (Variables|Default|GetXP)) " 
LEVEL" (Utilities|String|ToString(Integer) (Variables|Default|GetLevelPlayer))) true true "(R=0.000000,G=0.660000,B=1.000000,A=1.000000)" 1e+01))

(fn IncrementarLevel
  (params (AñadeLevel :type Integer) (Incrementar%20MaxExp :type Float%20%28double-precision%29))
  (Variables|Default|SetLevelPlayer (+ (Variables|Default|GetLevelPlayer) AñadeLevel))
  (Default|CallSuboNivel (Variables|Default|GetLevelPlayer))
  (Variables|Default|SetMax%20XP Incrementar%20MaxExp)
  (Variables|Default|SetXP (- (Variables|Default|GetXP) (Variables|Default|GetMax%20XP))))

(fn ExpInicial
  (Default|CallXPAlIniciar (Variables|Default|GetXP) (Variables|Default|GetMax%20XP)))

(fn LevelInicial
  (Default|CallLevIni (Variables|Default|GetLevelPlayer)))