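; BP_ComponenteVida is a health component that handles damage, healing and death for its owning actor.
; It broadcasts initial health one tick after BeginPlay and broadcasts again on non-lethal damage.
; Lethal damage reloads the current level if the owner is BP_Character.
; Healing clamps Vida without broadcasting, and Vida's OnRep refreshes the character's health bar.
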(event EventBeginPlay
  (Utilities|FlowControl|DelayUntilNextTick)
  (CallFunction|SaludInicial))

(event EventTick
  (params (DeltaSeconds :type Float%20%28single-precision%29)))

(event EventDanoesfera
  (params (dano :type Float%20%28double-precision%29))
  (CallFunction|DañoAlJugar dano))

(fn SaludInicial
  (Default|CallSaludIni (Variables|Default|GetVida) (Variables|Default|GetVida%20max)))

(fn DañoAlJugar
  (params (dano :type Float%20%28double-precision%29))
  (if (<= (Math|Float|Clamp(Float) (- (Variables|Default|GetVida) dano) 0.0 (Variables|Default|GetVida%20max)) 0.0)
    (Utilities|Casting|CastToBP_Character (Components|GetOwner))
    (bind _returnvalue (Game|GetCurrentLevelName true))
    (Game|OpenLevel(byName) (Utilities|String|StringToName _returnvalue))
    (else
      (Variables|Default|SetVida (Math|Float|Clamp(Float) (- (Variables|Default|GetVida) dano) 0.0 (Variables|Default|GetVida%20max)))
      (Default|CallRecibiDano (Variables|Default|GetVida) (Variables|Default|GetVida%20max)))))

(fn RecibirCuracion
  (params (Curar :type Float%20%28double-precision%29))
  (Variables|Default|SetVida (Math|Float|Clamp(Float) (+ Curar (Variables|Default|GetVida)) 0.0 (Variables|Default|GetVida%20max))))

(fn OnRepVida
  (bind _asbp_character (Utilities|Casting|CastToBP_Character (Components|GetOwner)))
  (Default|ActualizarUi _asbp_character (Variables|/Game/Characters/BP_Character.BP_Character_C|GetBarra%20de%20Vida _asbp_character)))

(fn OnRepVidaMax)