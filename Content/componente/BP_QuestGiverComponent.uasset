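; Quest-giver component that gives its owning actor one quest, set by the QuestData row handle, to offer and reward.
; InteractWith checks ComponenteMisiones on the player's PlayerState, then shows the offer widget, the reward widget or a debug print for completed or unfinished quests.
; Both widgets receive the quest's data table row, though the reward lookup uses a hardcoded DT_QuestData.
; When a widget is shown, it returns the owner's display name as objective ID.
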(event EventBeginPlay)

(event EventTick
  (params (DeltaSeconds :type Float%20%28single-precision%29)))

(fn DsiplayQuest
  (bind _questdata (Variables|Default|GetQuestData))
  (bind _returnvalue (Utilities|GetDataTableRow (.datatable _questdata) (.rowname _questdata))
    (:then
      (bind _returnvalue_2 (UserInterface|CreateWidget "/Game/ui/questUI/WBP_MisionesNPC.WBP_MisionesNPC_C" (Game|GetPlayerController 0) (.rowname _questdata) _returnvalue))
      (UserInterface|Viewport|AddtoViewport _returnvalue_2 0))))

(fn DisplayRecompensa
  (bind _questdata (Variables|Default|GetQuestData))
  (bind _returnvalue (Utilities|GetDataTableRow "/Game/Datatable/DT_QuestData.DT_QuestData" (.rowname _questdata))
    (:then
      (bind _returnvalue_2 (UserInterface|CreateWidget "/Game/ui/questUI/WBP_Recompensa.WBP_Recompensa_C" (Game|GetPlayerController 0) (.rowname _questdata) _returnvalue))
      (UserInterface|Viewport|AddtoViewport _returnvalue_2 0))))

(fn Interactwith
  (bind _returnvalue (Components|GetOwner))
  (bind _returnvalue_2 (Utilities|GetDisplayName _returnvalue))
  (bind _asplayer_state_countless_blood (Utilities|Casting|CastToPlayerStateCountlessBlood (Variables|/Script/Engine.Pawn|GetPlayerState (CallFunction|GetMyPlayerCharacter))))
  (if (Utilities|Array|ContainsItem (Variables|/Script/proyectoejercicio.ComponenteMisiones|GetCompletedQuests (Variables|/Script/proyectoejercicio.PlayerStateCountlessBlood|GetComponenteMisiones _asplayer_state_countless_blood)) (.rowname (Variables|Default|GetQuestData)))
    (Development|PrintString "MisionCompletada")
    (elif (not (Utilities|Array|ContainsItem (Variables|/Script/proyectoejercicio.ComponenteMisiones|GetActiveQuests (Variables|/Script/proyectoejercicio.PlayerStateCountlessBlood|GetComponenteMisiones _asplayer_state_countless_blood)) (.rowname (Variables|Default|GetQuestData))))
      (CallFunction|DsiplayQuest)
      (return (Utilities|String|StringToName _returnvalue_2) false)
      (elif (Class|ComponenteMisiones|IsQuestCompleted (Variables|/Script/proyectoejercicio.PlayerStateCountlessBlood|GetComponenteMisiones _asplayer_state_countless_blood) (.rowname (Variables|Default|GetQuestData)))
        (CallFunction|DisplayRecompensa)
        (return (Utilities|String|StringToName _returnvalue_2) false)
        (else
          (Development|PrintString "no termino la mision todavia" true true "(R=0.239583,G=0.000000,B=0.023937,A=1.000000)" 5.0))))))