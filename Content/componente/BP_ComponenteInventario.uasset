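; Inventory component that stores item quantities in the Content map and offers functions to add and query them.
; AnadirAlInventario increments an item's count and reports it to BP_Character as objective progress through CallOnObjetiveID.
; A separate helper just appends to Lista and prints the entry.
; The event graph's older slot-based inventory (widget toggle, eight slots, sphere-trace pickup with stacking) is disconnected and never runs.
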(event EventBeginPlay)

(event EventTick
  (params (DeltaSeconds :type Float%20%28single-precision%29)))

(event Input|KeyboardEvents|DebugKeyO
  (params (Key :type Key%20Structure :default "None") (ActionValue :type Input%20Action%20Value%20Structure)))

(event Input|KeyboardEvents|DebugKeyR
  (params (Key :type Key%20Structure :default "None") (ActionValue :type Input%20Action%20Value%20Structure)))

(fn AddItemstoinventory
  (params (NewItem :type String%20%28by%20ref%29))
  (Utilities|Array|Add (Variables|Default|Getlista) NewItem)
  (Development|PrintString NewItem))

(fn AnadirAlInventario
  (params (item :type Name) (cantidad :type Integer))
  (Utilities|Map|Add (Variables|Default|GetContent) item (+ cantidad (.Value (Utilities|Map|Find (Variables|Default|GetContent) item))))
  (bind _asbp_character (Utilities|Casting|CastToBP_Character (Game|GetPlayerCharacter 0)))
  (Default|CallOnObjetiveID _asbp_character (Utilities|String|ToString(Name) item) cantidad))

(fn QueryInventory
  (params (item :type Name))
  (return (.Value (Utilities|Map|Find (Variables|Default|GetContent) item))))