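; Inventory Blueprint that stores items as SItemData entries in an InventorySlots array.
; AddItem appends items not already present; for an exact match it rewrites the entry with the same values, leaving the stack count unchanged.
; The InventorySlots RepNotify calls OnInventoryUpdated to signal changes to listeners.
; Event graph and construction script are empty.
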(event EventBeginPlay)

(event Collision|EventActorBeginOverlap
  (params (OtherActor :type Actor%20Object%20Reference)))

(event EventTick
  (params (DeltaSeconds :type Float%20%28single-precision%29)))

(fn ConstructionScript)

(fn OnRepInventorySlots
  (Default|CallOnInventoryUpdated))

(fn AddItem
  (params (ItemToAdd :type S%20Item%20Data%20Structure))
  (bind _inventoryslots (Variables|Default|GetInventorySlots))
  (bind _inventoryslots_2 (Variables|Default|GetInventorySlots))
  (bind _returnvalue (Utilities|Array|FindItem _inventoryslots ItemToAdd))
  (bind _output (Utilities|Array|Get(acopy) _inventoryslots_2 _returnvalue))
  (if (>= _returnvalue 0)
    (Utilities|Array|SetArrayElem (Variables|Default|GetInventorySlots) _returnvalue (Utilities|Struct|MakeS_ItemData (.itemname _output) (.thumbnail _output) (.currentstack _output) (.maxstack _output)))
    (else
      (Utilities|Array|Add _inventoryslots_2 ItemToAdd))))